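; Lead bird actor whose Health represents the size of its flock and decides whether the game is won or lost.
; Overlapping a BP_CollectBird destroys it and adds Health, while overlapping a BP_Cloud destroys it and removes Health.
; Every tick, exact Health values open the lose level at zero or the win level at seven, and toggle visibility and collision on six flock components, which start hidden.
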(event EventTick
  (params (DeltaSeconds :type Float%20%28single-precision%29))
  (CallFunction|CheckWinLose)
  (CallFunction|ChangeFlockNumber))

(event Collision|EventActorBeginOverlap
  (params (OtherActor :type Actor%20Object%20Reference))
  (if (== (Utilities|GetClass OtherActor) "/Game/ActorsBlueprints/BP_CollectBird.BP_CollectBird_C")
    (Actor|DestroyActor OtherActor)
    (Variables|Default|SetHealth (+ (Variables|Default|GetHealth) 1.0))
    (elif (== (Utilities|GetClass OtherActor) "/Game/ActorsBlueprints/BP_Cloud.BP_Cloud_C")
      (Actor|DestroyActor OtherActor)
      (Variables|Default|SetHealth (+ (Variables|Default|GetHealth) -1.0)))))

(fn ConstructionScript
  (Rendering|SetVisibility (Variables|Default|GetFlock1) false false)
  (Collision|SetCollisionEnabled (Variables|Default|GetFlock1) "NoCollision"))

(fn ChangeFlockNumber
  (if (== (Variables|Default|GetHealth) 1.0)
    (Rendering|SetVisibility (Variables|Default|GetFlock1) false false)
    (Collision|SetCollisionEnabled (Variables|Default|GetFlock1) "NoCollision")
    (Rendering|SetVisibility (Variables|Default|GetBird) true false)
    (Collision|SetCollisionEnabled (Variables|Default|GetBird) "QueryAndPhysics")
    (elif (== (Variables|Default|GetHealth) 2.0)
      (Rendering|SetVisibility (Variables|Default|GetFlock2) false false)
      (Collision|SetCollisionEnabled (Variables|Default|GetFlock2) "NoCollision")
      (Rendering|SetVisibility (Variables|Default|GetFlock1) true false)
      (Collision|SetCollisionEnabled (Variables|Default|GetFlock1) "QueryAndPhysics")
      (elif (== (Variables|Default|GetHealth) 3.0)
        (Rendering|SetVisibility (Variables|Default|GetFlock3) false false)
        (Collision|SetCollisionEnabled (Variables|Default|GetFlock3) "NoCollision")
        (Rendering|SetVisibility (Variables|Default|GetFlock1) true false)
        (Collision|SetCollisionEnabled (Variables|Default|GetFlock1) "QueryAndPhysics")
        (elif (== (Variables|Default|GetHealth) 4.0)
          (Rendering|SetVisibility (Variables|Default|GetFlock4) false false)
          (Collision|SetCollisionEnabled (Variables|Default|GetFlock4) "NoCollision")
          (Rendering|SetVisibility (Variables|Default|GetFlock1) true false)
          (Collision|SetCollisionEnabled (Variables|Default|GetFlock1) "QueryAndPhysics")
          (elif (== (Variables|Default|GetHealth) 5.0)
            (Rendering|SetVisibility (Variables|Default|GetFlock5) false false)
            (Collision|SetCollisionEnabled (Variables|Default|GetFlock5) "NoCollision")
            (Rendering|SetVisibility (Variables|Default|GetFlock1) true false)
            (Collision|SetCollisionEnabled (Variables|Default|GetFlock1) "QueryAndPhysics")
            (elif (== (Variables|Default|GetHealth) 6.0)
              (Rendering|SetVisibility (Variables|Default|GetFlock6) false false)
              (Collision|SetCollisionEnabled (Variables|Default|GetFlock6) "NoCollision")
              (Rendering|SetVisibility (Variables|Default|GetFlock1) true false)
              (Collision|SetCollisionEnabled (Variables|Default|GetFlock1) "QueryAndPhysics")
              (elif (== (Variables|Default|GetHealth) 7.0)
                (Rendering|SetVisibility (Variables|Default|GetFlock1) true false)
                (Collision|SetCollisionEnabled (Variables|Default|GetFlock1) "QueryAndPhysics")))))))))

(fn CheckWinLose
  (if (== (Variables|Default|GetHealth) 0.0)
    (Game|OpenLevel(byName) "BP_Lose")
    (elif (== (Variables|Default|GetHealth) 7.0)
      (Game|OpenLevel(byName) "BP_Win"))))
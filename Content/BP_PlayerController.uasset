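; Player controller that moves the controlled pawn vertically in response to Up and Down inputs.
; Pressing either input sets a held flag and pitches the controller's own rotation from the value cached at BeginPlay, which is restored on release.
; Tick reads the flags to shift the pawn along Z by a fixed per-frame step without sweep or delta-time scaling, with Up taking priority.
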(event EventTick
  (params (DeltaSeconds :type Float%20%28single-precision%29))
  (bind _returnvalue (Pawn|GetControlledPawn))
  (bind _returnvalue_2 (Pawn|GetControlledPawn))
  (bind _returnvalue_3 (Transformation|GetActorLocation _returnvalue))
  (bind _returnvalue_4 (Transformation|GetActorLocation _returnvalue_2))
  (bind (_x _y _z) (Math|Vector|BreakVector _returnvalue_3))
  (bind (_x_2 _y_2 _z_2) (Math|Vector|BreakVector _returnvalue_4))
  (if (Variables|Default|GetUpPressed)
    ;[1 1 1] Move UP
    (Transformation|SetActorLocation _returnvalue_2 (Math|Vector|MakeVector _x_2 _y_2 (+ _z_2 1e+01)) false false)
    (elif (Variables|Default|GetDownPressed)
      ;[1 1 1] Move Down
      (Transformation|SetActorLocation _returnvalue (Math|Vector|MakeVector _x _y (+ _z -1e+01)) false false))))

(event EventBeginPlay
  (Variables|Default|SetOriginalRotation (Transformation|GetActorRotation)))

(event Input|ActionEvents|InputActionUp
  (params (Key :type Key%20Structure))
  (bind _originalrotation (Variables|Default|GetOriginalRotation))
  (bind (_roll _pitch _yaw) (Math|Rotator|BreakRotator _originalrotation))
  ;[1 1 1] Rotate Up
  (:Pressed
    (Variables|Default|SetUpPressed true)
    (Transformation|SetActorRotation (Math|Rotator|MakeRotator _roll (+ _pitch 1e+01) _yaw)))
  (:Released
    (Variables|Default|SetUpPressed false)
    (Transformation|SetActorRotation _originalrotation)))

(event Input|ActionEvents|InputActionDown
  (params (Key :type Key%20Structure))
  (bind _originalrotation (Variables|Default|GetOriginalRotation))
  (bind (_roll _pitch _yaw) (Math|Rotator|BreakRotator _originalrotation))
  ;[1 1 1] Rotate Down
  (:Pressed
    (Variables|Default|SetDownPressed true)
    (Transformation|SetActorRotation (Math|Rotator|MakeRotator _roll (+ _pitch -1e+01) _yaw)))
  (:Released
    (Variables|Default|SetDownPressed false)
    (Transformation|SetActorRotation _originalrotation)))

(fn ConstructionScript)